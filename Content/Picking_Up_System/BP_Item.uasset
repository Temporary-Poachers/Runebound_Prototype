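; BP_Item is a pickup item actor for the picking-up system, with its mesh set from a variable in the construction script.
; The PickUp event prints a debug message and plays a timeline that scales the root from full size to zero.
; The timeline's first update also starts a one-time short delay before the actor is destroyed.
; A separate PickUpItem function returns a hardcoded item name, "Pillar1".
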(event EventBeginPlay)

(event Collision|EventActorBeginOverlap
  (params (OtherActor :type Actor%20Object%20Reference)))

(event EventTick
  (params (DeltaSeconds :type Float%20%28single-precision%29)))

(event EventPickUp
  (Development|PrintString "Item Picked")
  (bind _shrinktimeline (Timeline|Shrink Play)
    (:Update
      (Transformation|SetWorldScale3D (Variables|Default|GetDefaultSceneRoot) (Math|Conversions|ToVector(Float) (Math|Float|Lerp 1.0 0.0 _shrinktimeline)))
      (Utilities|FlowControl|DoOnce false
        (:Completed
          (Utilities|FlowControl|Delay 0.4)
          (Actor|DestroyActor))))))

(fn ConstructionScript
  (Components|StaticMesh|SetStaticMesh (Variables|Default|GetItemModel) (Variables|Default|GetItemModelToPlace)))

(fn PickUpItem
  (return "Pillar1"))