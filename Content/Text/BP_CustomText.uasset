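; BP_CustomText is an actor that displays configurable 3D text in the world through a TextRender component.
; Its construction script applies the Font, FontSize, FontColor and Text variables to that component as font, world size, render color and content.
; The event graph holds only disabled default events, so the Blueprint adds no runtime logic.
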(event EventBeginPlay)

(event Collision|EventActorBeginOverlap
  (params (OtherActor :type Actor%20Object%20Reference)))

(event EventTick
  (params (DeltaSeconds :type Float%20%28single-precision%29)))

(fn ConstructionScript
  (Class|TextRenderComponent|SetFont (Variables|Default|GetTextRender) (Variables|Default|GetFont))
  (Rendering|Components|TextRender|SetWorldSize (Variables|Default|GetTextRender) (Variables|Default|GetFontSize))
  (Rendering|Components|TextRender|SetTextRenderColor (Variables|Default|GetTextRender) (Variables|Default|GetFontColor))
  (Rendering|Components|TextRender|SetText (Variables|Default|GetTextRender) (Variables|Default|GetText)))