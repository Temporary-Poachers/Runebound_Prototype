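; Custom pawn sensing component that lets a flying AI detect the first player's pawn and report visibility to its Blackboard.
; A looping timer runs SenseForTarget, which requires an unobstructed Visibility line trace, a hit within range and an angle inside the view cone around the component's forward vector.
; Each result updates the "CanSeeTarget?" key on the owner's AI controller, with optional cone drawing and failure messages for debugging.
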(event Custom|Begin%20Sensing
  ;[1 1 1] Begin sensing
  (bind _returnvalue (Utilities|Time|SetTimerbyEvent (delegate Custom|Sense) (Variables|Toggleable|GetSensingInterval) true))
  (Variables|Default|SetSensingTimerRef _returnvalue))

(event Custom|Sense
  ;[1 1 1] Sensing logic
  (bind _cansee_1 (CallFunction|SenseforTarget))
  (CallFunction|UpdateBBKey (AI|GetAIController (Components|GetOwner)) "CanSeeTarget?" "NewEnumerator0" _cansee_1 0 "0, 0, 0" 0.0))

(event Custom|Stop%20Sensing
  ;[1 1 1] Stop sensing
  (Utilities|Time|ClearandInvalidateTimerbyHandle (Variables|Default|GetSensingTimerRef)))

(event EventBeginPlay
  ;[1 1 1] Begin play
  (Variables|Default|SetTargetPawn (Game|Player|GetPlayerPawn 0))
  (CallFunction|BeginSensing))

(fn SenseforTarget
  (bind _returnvalue (Math|Vector|GetForwardVector))
  (bind _returnvalue_2 (Transformation|GetWorldLocation))
  (bind _pawnsensingconeangle (Variables|Toggleable|GetPawnSensingConeAngle))
  (bind _targetpawn (Variables|Default|GetTargetPawn))
  (bind _returnvalue_3 (Transformation|GetActorLocation _targetpawn))
  (bind _returnvalue_4 (Math|Vector|GetUnitDirection(Vector) _returnvalue_2 _returnvalue_3))
  (bind _returnvalue_5 (Math|Vector|DotProduct _returnvalue _returnvalue_4))
  (bind _returnvalue_6 (Class|KismetMathLibrary|DegAcos _returnvalue_5))
  (LocalVariables|SetCanSee? false)
  (if (Variables|Toggleable|GetDebug?)
    (Class|KismetSystemLibrary|DrawDebugConeinDegrees (.location (Transformation|GetWorldTransform)) (Math|Vector|GetForwardVector) (Variables|Toggleable|GetPawnSensingRange) _pawnsensingconeangle _pawnsensingconeangle 12 "(R=1.000000,G=1.000000,B=1.000000,A=1.000000)" (Variables|Toggleable|GetSensingInterval) 5.0))
  (bind (_outhit _returnvalue_7) (Collision|LineTraceByChannel (Transformation|GetWorldLocation) (Transformation|GetActorLocation (Variables|Default|GetTargetPawn)) "TraceTypeQuery1" false (Utilities|Array|MakeArray (Components|GetOwner)) (Variables|Toggleable|GetTraceDebugType)))
  (if _returnvalue_7
    (LocalVariables|SetCurrentHitResult _outhit)
    (if (== (.hitactor (LocalVariables|GetCurrentHitResult)) (Variables|Default|GetTargetPawn))
      (if (<= (.distance (LocalVariables|GetCurrentHitResult)) (Variables|Toggleable|GetPawnSensingRange))
        (if (<= _returnvalue_6 (Variables|Toggleable|GetPawnSensingConeAngle))
          (LocalVariables|SetCanSee? true)
          (return (LocalVariables|GetCanSee?))
          (else
            (CallFunction|DebugMessage (Utilities|String|Append "Pawn sensing: Target out of peripheral vision" "Angle = " (Utilities|String|ToString(Float) _returnvalue_6)))
            (return (LocalVariables|GetCanSee?))))
        (else
          (CallFunction|DebugMessage "Pawn sensing hit result was out of pawn sensing range")
          (return (LocalVariables|GetCanSee?))))
      (else
        (CallFunction|DebugMessage "Pawn sensing is blocked by an object")
        (return (LocalVariables|GetCanSee?))))
    (else
      (Development|PrintString "No hit from custom pawn sensing")
      (return (LocalVariables|GetCanSee?)))))

(fn DebugMessage
  (params (InString :type String))
  (if (Variables|Toggleable|GetDebug?)
    (Development|PrintString InString)))