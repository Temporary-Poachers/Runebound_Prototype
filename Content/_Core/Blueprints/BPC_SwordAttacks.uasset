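; Sword attack component for BP_ThirdPersonCharacterMixamo that runs a two-hit melee combo on the character mesh.
; SwordAttack starts a hit or buffers the press in SaveAttack, and SwordAttackCombo either plays the next hit or calls StopCombo to reset.
; Each hit plays its montage at AttackSpeed with a delayed swoosh, using DoOnce against re-entry.
; The IA_SwordAttack input event is empty, and the CanAttack check is unconnected.
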(event Custom|Sword%20Attack
  (if (Variables|Default|GetisAttacking?)
    (Variables|Default|SetSaveAttack true)
    (else
      (Variables|Default|SetisAttacking? true)
      (switch int (Variables|Default|GetAttack)
        (:0
          (CallFunction|SwordAttack1))
        (:1
          (CallFunction|SwordAttack2))))))

(event Custom|Stop%20Combo
  (Variables|Default|SetisAttacking? false)
  (Variables|Default|SetAttack 0))

(event Custom|Sword%20Attack%20Combo
  (if (Variables|Default|GetSaveAttack)
    (Variables|Default|SetSaveAttack false)
    (switch int (Variables|Default|GetAttack)
      (:0
        (CallFunction|SwordAttack1))
      (:1
        (CallFunction|SwordAttack2)))
    (else
      (CallFunction|StopCombo))))

(event Custom|Sword%20Attack%202
  ;[1 1 1] Sword Attack 2
  (Utilities|FlowControl|DoOnce false :!label _label
    (:Completed
      (Utilities|FlowControl|Delay 0.1)
      (Utilities|FlowControl|Sequence
        (:then_0
          (Animation|Montage|PlayMontage (Variables|Default|GetCharacterMesh) "/Game/_Core/Animations/SwordAttack_2_Montage.SwordAttack_2_Montage" (Variables|Default|GetAttackSpeed)
            (:then
              _)))
        (:then_1
          (Utilities|FlowControl|Delay 0.3)
          (Audio|PlaySound2D "/Game/_Core/Audio/Swoosh_Cue.Swoosh_Cue" 1.0 1.0 0.0 0 0)))
      (Variables|Default|SetAttack 2)
      (goto _label Reset))))

(event Custom|Sword%20Attack%201
  ;[1 1 1] Sword Attack 1
  (Utilities|FlowControl|DoOnce false :!label _label
    (:Completed
      (Utilities|FlowControl|Delay 0.1)
      (Utilities|FlowControl|Sequence
        (:then_0
          (Animation|Montage|PlayMontage (Variables|Default|GetCharacterMesh) "/Game/_Core/Animations/SwordAttack_1_Montage.SwordAttack_1_Montage" (Variables|Default|GetAttackSpeed)
            (:then
              _)))
        (:then_1
          (Utilities|FlowControl|Delay 0.3)
          (Audio|PlaySound2D "/Game/_Core/Audio/Swoosh_Cue.Swoosh_Cue" 1.0 1.0 0.0 0 0)))
      (Variables|Default|SetAttack 1)
      (goto _label Reset))))

(event Input|EnhancedActionEvents|EnhancedInputActionIA_SwordAttack
  (params (ActionValue :type Boolean) (ElapsedSeconds :type Float%20%28double-precision%29) (TriggeredSeconds :type Float%20%28double-precision%29) (InputAction :type Input%20Action%20Object%20Reference :default "/Game/Mixamo/ThirdPersonMixamo/Input/Actions/IA_SwordAttack.IA_SwordAttack")))

(event EventBeginPlay
  (bind _asbp_third_person_character_mixamo (Utilities|Casting|CastToBP_ThirdPersonCharacterMixamo (Components|GetOwner)))
  (Variables|Default|SetCharacterMesh (Variables|/Script/Engine.Character|GetMesh _asbp_third_person_character_mixamo)))