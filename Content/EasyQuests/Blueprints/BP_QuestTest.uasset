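; Test actor for the EasyQuests system that either advances active quest objectives or assigns new quests when play begins.
; After a short delay, it checks each listed quest's current objective against its objective IDs and adds one progress to matches through the Quest Component.
; If nothing matches, it starts its configured quests.
; A missing component only prints a message, and OnVisit is an empty stub.
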(event EventBeginPlay
  (bind (_componentwasfound_ _questcomponent) (CallFunction|GetQuestComponent))
  (if _componentwasfound_
    (Variables|Default|SetQuestComponent _questcomponent)
    (Utilities|FlowControl|Delay 0.2)
    (bind _out (CallFunction|CheckforAnyObjectives))
    (if (not _out)
      (Default|StartMultipleQuests (Variables|Default|GetQuestComponent) (Variables|Default|GetQuestsToAssign)))
    (else
      (Development|PrintString "Quest Component was not found." true true "(R=1.000000,G=0.052861,B=0.000000,A=1.000000)"))))

(event Collision|EventActorBeginOverlap
  (params (OtherActor :type Actor%20Object%20Reference)))

(event EventTick
  (params (DeltaSeconds :type Float%20%28single-precision%29)))

(event EventOnVisit
  (params (PlayerActor :type BP%20Third%20Person%20Character%20Mixamo%20Object%20Reference)))

(fn ConstructionScript)

(fn CheckforAnyObjectives
  (for _array_element (Variables|Default|GetQuest%20IDs)
    (if (.FoundObjective? (Default|GetCurrentObjectiveforActiveQuest (Variables|Default|GetQuestComponent) _array_element))
      (bind _array_element_2 (Utilities|Array|ForEachLoopwithBreak (Variables|Default|GetObjective%20IDs) :!label _label)
        (:LoopBody
          (if (Utilities|Name|Equal(Name) _array_element_2 (Utilities|Struct|BreakST_Quest_Objectives (.FoundObjectiveInfo (Default|GetCurrentObjectiveforActiveQuest (Variables|Default|GetQuestComponent) _array_element))))
            (Default|AddObjectiveAmount (Variables|Default|GetQuestComponent) _array_element _array_element_2 1)
            (LocalVariables|SetLocal%20Checked%20Any true)
            (goto _label Break))))))
  (return (LocalVariables|GetLocal%20Checked%20Any)))